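; Sliding door actor that opens when a Character overlaps its EnterTrigger.
; An IsDoorOpen flag guards the Opening and Closing events, which play the OpenDoor timeline forward or in reverse.
; The timeline value is mapped to the door's relative X location, with the X variable as upper bound.
; The ExitTrigger overlap is empty and its closing logic is disconnected, so nothing here closes the door.
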(event `self.EnterTrigger.OnComponentBeginOverlap`
  (params (OverlappedComponent :type "PrimitiveComponent Object Reference") (OtherActor :type "Actor Object Reference") (OtherComp :type "PrimitiveComponent Object Reference") (OtherBodyIndex :type Integer) (bFromSweep :type Boolean) (SweepResult :type "HitResult Structure (by ref)"))
  (cast `Character` OtherActor)
  (`self.Opening`))

(event `self.ExitTrigger.OnComponentBeginOverlap`
  (params (OverlappedComponent :type "PrimitiveComponent Object Reference") (OtherActor :type "Actor Object Reference") (OtherComp :type "PrimitiveComponent Object Reference") (OtherBodyIndex :type Integer) (bFromSweep :type Boolean) (SweepResult :type "HitResult Structure (by ref)")))

(event `Opening`
  (if (not (`self.isDoorOpen`))
    (set `self.isDoorOpen` true)
    (bind (_direction _zoffset) (`Timeline|OpenDoor` :!via `PlayFromStart` :!label _label)
      (:`Update`
        (`SceneComponent.K2_SetRelativeLocation` (`self.Door`) (`KismetMathLibrary.MakeVector` (`KismetMathLibrary.MapRangeClamped` _zoffset 0.0 1.0 0.0 (`self.X`))) false false)))))

(event `Closing`
  (if (`self.isDoorOpen`)
    (set `self.isDoorOpen` false)
    (goto _label :!via `ReverseFromEnd`)))

(fn `UserConstructionScript`)